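; Main game Blueprint for a 2D grid-based Snake game, spawning the HUD, snake head, food and border walls on BeginPlay.
; Tick runs a Delay-paced step that tests body and wall hits by location, handles eating, then reads gated direction input and shifts segments tail-to-head.
; Eating raises the score, grows the snake, respawns food and shortens the step delay.
; Collisions trigger game over, after which the restart input reloads the level.
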(event `Spawn New Snake Part`
  (params (`Spawn Location` :type "Vector Structure") (`Is Head` :type Boolean))
  ;[1 1 1] Спавн нового тела змейки
  (bind _returnvalue (`|SpawnActorFromClass` "/Game/Blueprints/BP_SnakeBodyPart.BP_SnakeBodyPart_C" (`KismetMathLibrary.MakeTransform` `Spawn Location`) "AlwaysSpawn" "OverrideRootScale" null null))
  (`PaperFlipbookComponent.SetFlipbook` (`/Game/Blueprints/BP_SnakeBodyPart.PaperFlipbook` _returnvalue) (select `bool` `Is Head` :`false` "/Game/Sprites/Flipbooks/FB_Step.FB_Step" :`true` "/Game/Sprites/Flipbooks/FB_Head.FB_Head" :!type "PaperFlipbook Object Reference"))
  (`KismetArrayLibrary.Array_Add` (`self.Snake Parts Array`) _returnvalue)
  (set `/Game/Blueprints/BP_SnakeBodyPart.Is Head` `Is Head` _returnvalue)
  (`self.K2_SetActorRotation` _returnvalue (`KismetMathLibrary.MakeRotator` 0.0) false))

(event `Spawn Food`
  (bind _returnvalue (- (`self.X_Max`) 100.0))
  (bind _returnvalue_2 (- (`self.Z_Max`) 100.0))
  ;[1 1 1] Спавн еды
  (bind _returnvalue_3 (`|SpawnActorFromClass` "/Game/Blueprints/BP_Food.BP_Food_C" (`KismetMathLibrary.MakeTransform` (`KismetMathLibrary.MakeVector` (* (`.ReturnValue` (`KismetMathLibrary.FMod` (`KismetMathLibrary.RandomFloatInRange` (* _returnvalue -1.0) _returnvalue) 100.0)) 100.0) -0.1 (* (`.ReturnValue` (`KismetMathLibrary.FMod` (`KismetMathLibrary.RandomFloatInRange` (* _returnvalue_2 -1.0) _returnvalue_2) 100.0)) 100.0))) "AlwaysSpawn" "OverrideRootScale" null null))
  (set `self.Food Actor REF` _returnvalue_3))

(event `Kill Snake`
  ;[1 1 1] Проверка на смерть
  (set `self.Is Dead` true)
  (for (_array_element _array_index) (`self.Snake Parts Array`)
    (`PaperFlipbookComponent.SetFlipbook` (`/Game/Blueprints/BP_SnakeBodyPart.PaperFlipbook` _array_element) (select `bool` (== _array_index 0) :`false` "/Game/Sprites/Flipbooks/FB_Head.FB_Head" :`true` "/Game/Sprites/Flipbooks/FB_Step.FB_Step" :!type "PaperFlipbook Object Reference")))
  (`KismetSystemLibrary.Delay` 0.5)
  (for _array_element_2 (`self.Snake Parts Array`)
    (`PaperFlipbookComponent.SetFlipbook` (`/Game/Blueprints/BP_SnakeBodyPart.PaperFlipbook` _array_element_2) null)))

(event `Update Score`
  (params (Value :type Integer))
  ;[1 1 1] Обновление сетчика
  (bind _output_get (set `self.Score` (+ Value (`self.Score`))))
  (`/Game/Blueprints/BP_UI_HUD.Update Score` (`self.HUD REF`) _output_get))

(event `self.ReceiveBeginPlay`
  (bind (_remainder _returnvalue) (`KismetMathLibrary.FMod` (`self.Z_Max`) 50.0))
  (bind (_remainder_2 _returnvalue_2) (`KismetMathLibrary.FMod` (`self.X_Max`) 50.0))
  ;[1 1 1] Определение параметров
  (bind _returnvalue_3 (`|CreateWidget` "/Game/Blueprints/BP_UI_HUD.BP_UI_HUD_C"))
  (bind _output_get (set `self.HUD REF` _returnvalue_3))
  (`UserWidget.AddToViewport` _output_get 0)
  (switch `int` (`KismetMathLibrary.RandomInteger` 3)
    (:`0`
      (set `self.Direction X` 1))
    (:`1`
      (set `self.Direction X` -1))
    (:`2`
      (set `self.Direction Z` 1))
    (:`3`
      (set `self.Direction Z` -1)))
  (set `self.Delay` 0.15)
  (`KismetArrayLibrary.Array_Clear` (`self.Snake Parts Array`))
  (`self.Spawn New Snake Part` (0.0 0.0 0.0) true)
  (`self.Spawn Food`)
  (for _index (range (* _returnvalue_2 _returnvalue))
    (bind _returnvalue_4 (/ _index _returnvalue))
    (bind _returnvalue_5 (mod _index _returnvalue))
    (if (or (== _returnvalue_4 0) (== _returnvalue_4 (- _returnvalue_2 1)) (== _returnvalue_5 0) (== _returnvalue_5 (- _returnvalue 1)))
      (bind _returnvalue_6 (`|SpawnActorFromClass` "/Game/Blueprints/BP_Block.BP_Block_C" (`KismetMathLibrary.MakeTransform` (`KismetMathLibrary.MakeVector` (+ (* (`self.X_Max`) -1.0) (* _returnvalue_4 100.0)) 0.0 (+ (* (`self.Z_Max`) -1.0) (* _returnvalue_5 100.0)))) "AdjustIfPossibleButDontSpawnIfColliding" "OverrideRootScale" null null))
      (`KismetArrayLibrary.Array_Add` (`self.Wall Blocks Array`) _returnvalue_6))))

(event `InputAction|RESTART`
  (params (Key :type "Key Structure"))
  ;[1 0.5971 0.2451] Весь процесс игры/  Все кнопки прописаны в пути: Edit -> Project Settings -> Input -> Action Mappings
  (:`Pressed`
    (goto _label :!via `Open`)))

(event `InputAction|QUITE`
  (params (Key :type "Key Structure"))
  ;[1 0.5971 0.2451] Весь процесс игры/  Все кнопки прописаны в пути: Edit -> Project Settings -> Input -> Action Mappings
  ;;[1 1 1] Выход из игры
  (:`Pressed`
    (`KismetSystemLibrary.QuitGame` null "Quit")))

(event `self.ReceiveTick`
  (params (DeltaSeconds :type "Float (single-precision)"))
  (bind _snake_parts_array (`self.Snake Parts Array`))
  ;[1 0.5971 0.2451] Весь процесс игры/  Все кнопки прописаны в пути: Edit -> Project Settings -> Input -> Action Mappings
  (if (`self.Is Dead`)
    (`/Engine/EditorBlueprintResources/StandardMacros.Gate` true :!label _label
      (:`Exit`
        (`/Engine/EditorBlueprintResources/StandardMacros.DoOnce` false
          (:`Completed`
            (`Widget.RemoveFromParent` (`self.HUD REF`))
            (bind _returnvalue (`GameplayStatics.GetCurrentLevelName` true))
            (`GameplayStatics.OpenLevel` (`KismetStringLibrary.Conv_StringToName` _returnvalue))))))
    (else
      (`KismetSystemLibrary.Delay` (`self.Delay`))
      (`|ExecutionSequence`
        (:`then_0`
          (for (_array_element _array_index) (`self.Snake Parts Array`) :!label _label_2
            (if (!= _array_index 0)
              (if (== (`self.K2_GetActorLocation` _array_element) (`self.K2_GetActorLocation` (`|GetArrayItem` (`self.Snake Parts Array`))))
                (`GameplayStatics.PlaySound2D` "/Game/Sound/bomb.bomb" 1.0 1.0 0.0 null null)
                (`self.Kill Snake`)
                (`/Game/Blueprints/BP_UI_HUD.Game Over Event` (`self.HUD REF`))
                (`self.Break Self Collision Test Loop`))))
          (for _array_element_2 (`self.Wall Blocks Array`) :!label _label_3
            (if (== (`self.K2_GetActorLocation` _array_element_2) (`self.K2_GetActorLocation` (`|GetArrayItem` (`self.Snake Parts Array`))))
              (`GameplayStatics.PlaySound2D` "/Game/Sound/bomb.bomb" 1.0 1.0 0.0 null null)
              (`self.Kill Snake`)
              (`/Game/Blueprints/BP_UI_HUD.Game Over Event` (`self.HUD REF`))
              (`self.Break Wall Collision Test Loop`))))
        (:`then_1`
          (if (not (`self.Is Dead`))
            (`|ExecutionSequence`
              (:`then_0`
                (if (== (`self.K2_GetActorLocation` (`|GetArrayItem` (`self.Snake Parts Array`))) (`self.K2_GetActorLocation` (`self.Food Actor REF`)) :`ErrorTolerance` 1.0)
                  (`GameplayStatics.PlaySound2D` "/Game/Sound/hrust.hrust" 1.0 1.0 0.0 null null)
                  (`self.Update Score` (`/Game/Blueprints/BP_Food.Score` (`self.Food Actor REF`)))
                  (`self.K2_DestroyActor` (`self.Food Actor REF`))
                  (`self.Spawn New Snake Part` (`self.K2_GetActorLocation` (`|GetArrayItem` _snake_parts_array (`KismetArrayLibrary.Array_LastIndex` _snake_parts_array))))
                  (`self.Spawn Food`)
                  (set `self.Delay` (`KismetMathLibrary.FClamp` (+ (`self.Delay`) -0.01) 0.075 0.2))))
              (:`then_1`
                (`|ExecutionSequence`
                  (:`then_0`
                    (`/Engine/EditorBlueprintResources/StandardMacros.Gate` true :!label _label_4
                      (:`Exit`
                        (if (and (== (`self.Direction Z`) 0) (`self.Can Change Direction`))
                          (set `self.Direction X` 0)
                          (set `self.Direction Z` 1)
                          (set `self.Can Change Direction` false :!label _label_5)))))
                  (:`then_1`
                    (`/Engine/EditorBlueprintResources/StandardMacros.Gate` true :!label _label_6
                      (:`Exit`
                        (if (and (== (`self.Direction Z`) 0) (`self.Can Change Direction`))
                          (set `self.Direction X` 0)
                          (set `self.Direction Z` -1)
                          (goto _label_5)))))
                  (:`then_2`
                    (`/Engine/EditorBlueprintResources/StandardMacros.Gate` true :!label _label_7
                      (:`Exit`
                        (if (and (== (`self.Direction X`) 0) (`self.Can Change Direction`))
                          (set `self.Direction X` 1)
                          (set `self.Direction Z` 0)
                          (goto _label_5)))))
                  (:`then_3`
                    (`/Engine/EditorBlueprintResources/StandardMacros.Gate` true :!label _label_8
                      (:`Exit`
                        (if (and (== (`self.Direction X`) 0) (`self.Can Change Direction`))
                          (set `self.Direction X` -1)
                          (set `self.Direction Z` 0)
                          (goto _label_5)))))
                  (:`then_4`
                    (for _index (range (`KismetArrayLibrary.Array_Length` (`self.Snake Parts Array`)))
                      (bind _returnvalue_2 (- (- (`KismetArrayLibrary.Array_Length` (`self.Snake Parts Array`)) 1) _index))
                      (if (`/Game/Blueprints/BP_SnakeBodyPart.Is Head` (`|GetArrayItem` (`self.Snake Parts Array`) _returnvalue_2))
                        (bind _output (`|GetArrayItem` (`self.Snake Parts Array`) _returnvalue_2))
                        (`self.K2_AddActorWorldOffset` _output (`KismetMathLibrary.MakeVector` (* (`self.Direction X`) 100.0) 0.0 (* (`self.Direction Z`) 100.0)) false false)
                        (else
                          (`self.K2_SetActorLocation` _output (`self.K2_GetActorLocation` (`|GetArrayItem` (`self.Snake Parts Array`) (- _returnvalue_2 1))) false false))))
                    (set `self.Can Change Direction` true)))))))))))

(event `Break Self Collision Test Loop`
  ;[1 0.5971 0.2451] Весь процесс игры/  Все кнопки прописаны в пути: Edit -> Project Settings -> Input -> Action Mappings
  (goto _label_2 :!via `Break`))

(event `Break Wall Collision Test Loop`
  ;[1 0.5971 0.2451] Весь процесс игры/  Все кнопки прописаны в пути: Edit -> Project Settings -> Input -> Action Mappings
  (goto _label_3 :!via `Break`))

(event `InputAction|UP`
  (params (Key :type "Key Structure"))
  ;[1 0.5971 0.2451] Весь процесс игры/  Все кнопки прописаны в пути: Edit -> Project Settings -> Input -> Action Mappings
  (:`Pressed`
    (goto _label_4 :!via `Open`))
  (:`Released`
    (goto _label_4 :!via `Close`)))

(event `InputAction|DOWN`
  (params (Key :type "Key Structure"))
  ;[1 0.5971 0.2451] Весь процесс игры/  Все кнопки прописаны в пути: Edit -> Project Settings -> Input -> Action Mappings
  (:`Pressed`
    (goto _label_6 :!via `Open`))
  (:`Released`
    (goto _label_6 :!via `Close`)))

(event `InputAction|RIGHT`
  (params (Key :type "Key Structure"))
  ;[1 0.5971 0.2451] Весь процесс игры/  Все кнопки прописаны в пути: Edit -> Project Settings -> Input -> Action Mappings
  (:`Pressed`
    (goto _label_7 :!via `Open`))
  (:`Released`
    (goto _label_7 :!via `Close`)))

(event `InputAction|LEFT`
  (params (Key :type "Key Structure"))
  ;[1 0.5971 0.2451] Весь процесс игры/  Все кнопки прописаны в пути: Edit -> Project Settings -> Input -> Action Mappings
  (:`Pressed`
    (goto _label_8 :!via `Open`))
  (:`Released`
    (goto _label_8 :!via `Close`)))

(fn `UserConstructionScript`)