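; BP_Food is a food object that keeps changing its type, updating its sprite and Score value.
; BeginPlay starts SetFood, which applies a type, waits a type-specific delay, then calls itself again indefinitely.
; Higher-scoring types stay longer.
; SetFood ignores its Type input and rolls its own random pick, and the Red and Yellow branches are identical.
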(event `self.ReceiveBeginPlay`
  (`self.Set Food` "NewEnumerator0"))

(event `Set Food`
  (params (Type :type "/Game/Blueprints/FoodColor_Enum Enum" :default "NewEnumerator0"))
  (bind _food_sprite (`self.Food Sprite`))
  (bind _outitem (`KismetArrayLibrary.Array_Random` (`|MakeArray` "NewEnumerator0" "NewEnumerator1" "NewEnumerator2" "NewEnumerator3" :!type "/Game/Blueprints/FoodColor_Enum Enum")))
  (switch `/Game/Blueprints/FoodColor_Enum` _outitem
    (:`NewEnumerator0`
      (`PaperSpriteComponent.SetSprite` _food_sprite "/Game/Sprites/BluePolygon_Sprite.BluePolygon_Sprite")
      (set `self.Score` 10)
      (`KismetSystemLibrary.Delay` 3.0)
      (`self.Set Food` _outitem))
    (:`NewEnumerator1`
      (`PaperSpriteComponent.SetSprite` _food_sprite "/Game/Sprites/S_Cake.S_Cake")
      (set `self.Score` 5)
      (`KismetSystemLibrary.Delay` 2.0)
      (`self.Set Food` _outitem))
    (:`NewEnumerator2`
      (`PaperSpriteComponent.SetSprite` _food_sprite "/Game/Sprites/S_RedA.S_RedA")
      (set `self.Score` 2)
      (`KismetSystemLibrary.Delay` 1.0)
      (`self.Set Food` _outitem))
    (:`NewEnumerator3`
      (`PaperSpriteComponent.SetSprite` _food_sprite "/Game/Sprites/S_RedA.S_RedA")
      (set `self.Score` 2)
      (`KismetSystemLibrary.Delay` 1.0)
      (`self.Set Food` _outitem))))

(fn `UserConstructionScript`)